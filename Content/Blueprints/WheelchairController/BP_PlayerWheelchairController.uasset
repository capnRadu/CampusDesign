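; Player controller for a Chaos-vehicle wheelchair that simulates manual hand pushes and routes Enhanced Input to the pawn.
; Held throttle inputs and forward speed select Idle, Forward, Backward or Brake, with opposing input braking first.
; Looping timers apply rear-wheel torque directly: speed-capped drive pulses with push animations, or sustained braking.
; It also handles steering, look, interaction, camera switching, goal skipping, menu exit and single- or double-press reset (wheelchair or checkpoint).
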(event `self.ReceiveBeginPlay`
  (`|ExecutionSequence`
    (:`then_0`
      (bind _asbp_player_wheelchair (cast `/Game/Blueprints/WheelchairController/BP_PlayerWheelchair` (`self.K2_GetPawn`)))
      (set `self.BP_PlayerWheelchair` _asbp_player_wheelchair))
    (:`then_1`
      (bind _aschaos_wheeled_vehicle_movement_component (cast `ChaosWheeledVehicleMovementComponent` (`WheeledVehiclePawn.VehicleMovementComponent` (`self.BP_PlayerWheelchair`))))
      (set `self.WheelchairVehicleMovementComponent` _aschaos_wheeled_vehicle_movement_component)
      (`self.SetVehicleMovementDefaults`))
    (:`then_2`
      (`EnhancedInputSubsystemInterface.AddMappingContext` (pcsubsystem `EnhancedInputLocalPlayerSubsystem` self) "/Game/Input/Wheelchair/IMC_PlayerWheelchair.IMC_PlayerWheelchair" 0 (struct)))))

(event `SetVehicleMovementDefaults`
  (bind _wheelchairvehiclemovementcomponent (`self.WheelchairVehicleMovementComponent`))
  (bind _wheelchairvehiclemovementcomponent_2 (`self.WheelchairVehicleMovementComponent`))
  (bind _wheelchairvehiclemovementcomponent_3 (`self.WheelchairVehicleMovementComponent`))
  (`ChaosWheeledVehicleMovementComponent.SetTorqueCombineMethod` _wheelchairvehiclemovementcomponent "Override" 2)
  (`ChaosWheeledVehicleMovementComponent.SetTorqueCombineMethod` _wheelchairvehiclemovementcomponent "Override" 3)
  (`ChaosWheeledVehicleMovementComponent.SetAffectedByHandbrake` _wheelchairvehiclemovementcomponent_2 2 false)
  (`ChaosWheeledVehicleMovementComponent.SetAffectedByHandbrake` _wheelchairvehiclemovementcomponent_2 3 false)
  (`ChaosWheeledVehicleMovementComponent.SetAffectedByHandbrake` _wheelchairvehiclemovementcomponent_3 0 false)
  (`ChaosWheeledVehicleMovementComponent.SetAffectedByHandbrake` _wheelchairvehiclemovementcomponent_3 1 false))

(event `EnhancedInput|/Game/Input/Wheelchair/Actions/IA_ThrottleUp`
  (params (ActionValue :type "Float (double-precision)") (ElapsedSeconds :type "Float (double-precision)") (TriggeredSeconds :type "Float (double-precision)") (InputAction :type "InputAction Object Reference" :default "/Game/Input/Wheelchair/Actions/IA_ThrottleUp.IA_ThrottleUp"))
  ; Manual wheelchair movement logic
  (:`Triggered`
    (`self.EvaluateMovement` :!label _label))
  (:`Started`
    (set `self.ThrottleUpHeld` true)
    (goto _label))
  (:`Completed`
    (set `self.ThrottleUpHeld` false)
    (goto _label)))

(event `EnhancedInput|/Game/Input/Wheelchair/Actions/IA_SteeringLeft`
  (params (ActionValue :type "Float (double-precision)") (ElapsedSeconds :type "Float (double-precision)") (TriggeredSeconds :type "Float (double-precision)") (InputAction :type "InputAction Object Reference" :default "/Game/Input/Wheelchair/Actions/IA_SteeringLeft.IA_SteeringLeft"))
  ; Other inputs
  (:`Triggered`
    (`ChaosVehicleMovementComponent.SetSteeringInput` (`WheeledVehiclePawn.VehicleMovementComponent` (`self.BP_PlayerWheelchair`)) ActionValue :!label _label_2))
  (:`Completed`
    (goto _label_2)))

(event `EnhancedInput|/Game/Input/Wheelchair/Actions/IA_LookY`
  (params (ActionValue :type "Float (double-precision)") (ElapsedSeconds :type "Float (double-precision)") (TriggeredSeconds :type "Float (double-precision)") (InputAction :type "InputAction Object Reference" :default "/Game/Input/Wheelchair/Actions/IA_LookY.IA_LookY"))
  ; Other inputs
  (:`Triggered`
    (`Pawn.AddControllerPitchInput` (`self.BP_PlayerWheelchair`) (* ActionValue (`self.MouseSensitivity`)))))

(event `EnhancedInput|/Game/Input/Wheelchair/Actions/IA_ThrottleUp`
  (params (ActionValue :type "Float (double-precision)") (ElapsedSeconds :type "Float (double-precision)") (TriggeredSeconds :type "Float (double-precision)") (InputAction :type "InputAction Object Reference" :default "/Game/Input/Wheelchair/Actions/IA_ThrottleUp.IA_ThrottleUp"))
  ;[0.15 0.02187 0.02187 0.5] Automatic wheelchair movement logic
)

(event `EnhancedInput|/Game/Input/Wheelchair/Actions/IA_SteeringRight`
  (params (ActionValue :type "Float (double-precision)") (ElapsedSeconds :type "Float (double-precision)") (TriggeredSeconds :type "Float (double-precision)") (InputAction :type "InputAction Object Reference" :default "/Game/Input/Wheelchair/Actions/IA_SteeringRight.IA_SteeringRight"))
  ; Other inputs
  (:`Triggered`
    (`ChaosVehicleMovementComponent.SetSteeringInput` (`WheeledVehiclePawn.VehicleMovementComponent` (`self.BP_PlayerWheelchair`)) ActionValue :!label _label_3))
  (:`Completed`
    (goto _label_3)))

(event `EnhancedInput|/Game/Input/Wheelchair/Actions/IA_LookX`
  (params (ActionValue :type "Float (double-precision)") (ElapsedSeconds :type "Float (double-precision)") (TriggeredSeconds :type "Float (double-precision)") (InputAction :type "InputAction Object Reference" :default "/Game/Input/Wheelchair/Actions/IA_LookX.IA_LookX"))
  ; Other inputs
  (:`Triggered`
    (`Pawn.AddControllerYawInput` (`self.BP_PlayerWheelchair`) (* ActionValue (`self.MouseSensitivity`)))))

(event `EnhancedInput|/Game/Input/Wheelchair/Actions/IA_ThrottleDown`
  (params (ActionValue :type "Float (double-precision)") (ElapsedSeconds :type "Float (double-precision)") (TriggeredSeconds :type "Float (double-precision)") (InputAction :type "InputAction Object Reference" :default "/Game/Input/Wheelchair/Actions/IA_ThrottleDown.IA_ThrottleDown"))
  ;[0.15 0.02187 0.02187 0.5] Automatic wheelchair movement logic
)

(event `EnhancedInput|/Game/Input/Wheelchair/Actions/IA_ThrottleDown`
  (params (ActionValue :type "Float (double-precision)") (ElapsedSeconds :type "Float (double-precision)") (TriggeredSeconds :type "Float (double-precision)") (InputAction :type "InputAction Object Reference" :default "/Game/Input/Wheelchair/Actions/IA_ThrottleDown.IA_ThrottleDown"))
  ; Manual wheelchair movement logic
  (:`Triggered`
    (`self.EvaluateMovement` :!label _label_4))
  (:`Started`
    (set `self.ThrottleDownHeld` true)
    (goto _label_4))
  (:`Completed`
    (set `self.ThrottleDownHeld` false)
    (goto _label_4)))

(event `EnhancedInput|/Game/Input/IA_Interact`
  (params (ActionValue :type Boolean) (ElapsedSeconds :type "Float (double-precision)") (TriggeredSeconds :type "Float (double-precision)") (InputAction :type "InputAction Object Reference" :default "/Game/Input/IA_Interact.IA_Interact"))
  ; Other inputs
  (:`Started`
    (`/Game/Blueprints/WheelchairController/BP_PlayerWheelchair.TryInteract` (`self.BP_PlayerWheelchair`))))

(event `EnhancedInput|/Game/Input/Wheelchair/Actions/IA_SwitchCamera`
  (params (ActionValue :type Boolean) (ElapsedSeconds :type "Float (double-precision)") (TriggeredSeconds :type "Float (double-precision)") (InputAction :type "InputAction Object Reference" :default "/Game/Input/Wheelchair/Actions/IA_SwitchCamera.IA_SwitchCamera"))
  ; Other inputs
  (:`Started`
    (`/Game/Blueprints/WheelchairController/BP_PlayerWheelchair.ChangeCamera` (`self.BP_PlayerWheelchair`))))

(event `EnhancedInput|/Game/Input/Wheelchair/Actions/IA_Brake`
  (params (ActionValue :type "Float (double-precision)") (ElapsedSeconds :type "Float (double-precision)") (TriggeredSeconds :type "Float (double-precision)") (InputAction :type "InputAction Object Reference" :default "/Game/Input/Wheelchair/Actions/IA_Brake.IA_Brake"))
  ;[0.15 0.02187 0.02187 0.5] Automatic wheelchair movement logic
)

(event `EvaluateMovement`
  ; Manual wheelchair movement logic
  (bind _desiredmode (`self.DetermineDesiredMovementMode`))
  (if (`|EnumInequality` _desiredmode (`self.CurrentMovementMode`))
    (if (or (`|EnumEquality` _desiredmode "NewEnumerator1") (`|EnumEquality` _desiredmode "NewEnumerator2"))
      (`KismetSystemLibrary.Delay` 0.2))
    (`self.EnterMovementMode` _desiredmode)))

(event `EnhancedInput|/Game/Input/IA_Exit`
  (params (ActionValue :type Boolean) (ElapsedSeconds :type "Float (double-precision)") (TriggeredSeconds :type "Float (double-precision)") (InputAction :type "InputAction Object Reference" :default "/Game/Input/IA_Exit.IA_Exit"))
  ; Other inputs
  (:`Started`
    (`GameplayStatics.OpenLevel` "MainMenu")))

(event `EnhancedInput|/Game/Input/IA_SkipGoal`
  (params (ActionValue :type Boolean) (ElapsedSeconds :type "Float (double-precision)") (TriggeredSeconds :type "Float (double-precision)") (InputAction :type "InputAction Object Reference" :default "/Game/Input/IA_SkipGoal.IA_SkipGoal"))
  ; Other inputs
  (:`Started`
    (`/Game/Blueprints/WheelchairController/BP_PlayerWheelchair.SkipCurrentGoal` (`self.BP_PlayerWheelchair`))))

(event `Drive`
  (params (DirectionSign :type "Float (double-precision)"))
  (bind _skm_character (`/Game/Blueprints/WheelchairController/BP_PlayerWheelchair.SKM_Character` (`self.BP_PlayerWheelchair`)))
  ; Manual wheelchair movement logic
  (if (not (`KismetSystemLibrary.K2_IsValidTimerHandle` (`self.PushTimer`)))
    (`self.CancelBrakeTorque`)
    (bind _returnvalue (`KismetSystemLibrary.K2_SetTimerDelegate` (delegate `Push`) 0.5 true))
    (set `self.PushTimer` _returnvalue)
    (bind _forwardspeed (`self.GetForwardSpeed` :!label _label_5))
    (if (< (`KismetMathLibrary.Abs` _forwardspeed) (`self.MaxSpeed`))
      (`self.SetRearDriveTorque` (* DirectionSign (`self.DriveTorque`)))
      (`|ExecutionSequence`
        (:`then_0`
          (if (`SkeletalMeshComponent.IsPlaying` _skm_character)
            _
            (elif (== DirectionSign 1.0)
              (`SkeletalMeshComponent.PlayAnimation` _skm_character "/Game/Art/Models/CharacterPlaceholder/Push_Forward_Anim.Push_Forward_Anim" false)
              (else
                (`SkeletalMeshComponent.PlayAnimation` _skm_character "/Game/Art/Models/CharacterPlaceholder/Push_Backward_Anim.Push_Backward_Anim" false)))))
        (:`then_1`
          (`KismetSystemLibrary.Delay` 0.1)
          (`self.SetRearDriveTorque` 0.0))))))

(event `self.ReceiveTick`
  (params (DeltaSeconds :type "Float (single-precision)")))

(event `EnhancedInput|/Game/Input/Wheelchair/Actions/IA_Reset`
  (params (ActionValue :type Boolean) (ElapsedSeconds :type "Float (double-precision)") (TriggeredSeconds :type "Float (double-precision)") (InputAction :type "InputAction Object Reference" :default "/Game/Input/Wheelchair/Actions/IA_Reset.IA_Reset"))
  ; Other inputs
  (:`Started`
    (if (`self.WaitingForSecondPress`)
      (`KismetSystemLibrary.K2_ClearAndInvalidateTimerHandle` (`self.DoublePressTimer`))
      (set `self.WaitingForSecondPress` false)
      (`/Game/Blueprints/WheelchairController/BP_PlayerWheelchair.ResetFromLastCheckpoint` (`self.BP_PlayerWheelchair`))
      (else
        (set `self.WaitingForSecondPress` true)
        (bind _returnvalue (`KismetSystemLibrary.K2_SetTimerDelegate` (delegate `SinglePressConfirmed`) (`self.DoublePressTime`)))
        (set `self.DoublePressTimer` _returnvalue)))))

(event `Push`
  ; Manual wheelchair movement logic
  (goto _label_5))

(event `ApplyBrake`
  (params (DesiredBrakeTorque :type "Float (double-precision)"))
  ; Manual wheelchair movement logic
  (if (not (`KismetSystemLibrary.K2_IsValidTimerHandle` (`self.BrakeTimer`)))
    (`self.CancelDriveTorque`)
    (bind _returnvalue (`KismetSystemLibrary.K2_SetTimerDelegate` (delegate `Brake`) 0.05 true))
    (set `self.BrakeTimer` _returnvalue)
    (`self.SetRearBrakeTorque` DesiredBrakeTorque :!label _label_6)))

(event `SinglePressConfirmed`
  ; Other inputs
  (set `self.WaitingForSecondPress` false)
  (`/Game/Blueprints/WheelchairController/BP_PlayerWheelchair.ResetWheelchair` (`self.BP_PlayerWheelchair`)))

(event `Brake`
  ; Manual wheelchair movement logic
  (goto _label_6))

(event `CancelBrakeTorque`
  ; Manual wheelchair movement logic
  (`KismetSystemLibrary.K2_ClearAndInvalidateTimerHandle` (`self.BrakeTimer`))
  (`self.SetRearBrakeTorque` 0.0))

(event `CancelDriveTorque`
  ; Manual wheelchair movement logic
  (`KismetSystemLibrary.K2_ClearAndInvalidateTimerHandle` (`self.PushTimer`))
  (`self.SetRearDriveTorque` 0.0))

(fn `DetermineDesiredMovementMode`
  (returns (DesiredMode :type "/Game/Blueprints/WheelchairController/E_MovementMode Enum"))
  (bind _forwardspeed (`self.GetForwardSpeed`))
  (if (and (`self.ThrottleUpHeld`) (not (`self.ThrottleDownHeld`)))
    (if (< _forwardspeed (* (`self.StopThreshold`) -1.0))
      (return "NewEnumerator3")
      (else
        (return "NewEnumerator1")))
    (elif (and (`self.ThrottleDownHeld`) (not (`self.ThrottleUpHeld`)))
      (if (> _forwardspeed (`self.StopThreshold`))
        (return "NewEnumerator3")
        (else
          (return "NewEnumerator2")))
      (else
        (return "NewEnumerator0")))))

(fn `EnterMovementMode`
  (params (NewMode :type "/Game/Blueprints/WheelchairController/E_MovementMode Enum" :default "NewEnumerator0"))
  (switch `/Game/Blueprints/WheelchairController/E_MovementMode` NewMode
    (:`NewEnumerator0`
      (`self.ApplyBrake` (`self.IdleBrakeTorque`))
      (`self.CancelDriveTorque`)
      (set `self.CurrentMovementMode` "NewEnumerator0"))
    (:`NewEnumerator1`
      (`self.Drive` 1.0)
      (set `self.CurrentMovementMode` "NewEnumerator1"))
    (:`NewEnumerator2`
      (`self.Drive` -1.0)
      (set `self.CurrentMovementMode` "NewEnumerator2"))
    (:`NewEnumerator3`
      (`self.ApplyBrake` (`self.BrakeTorque`))
      (set `self.CurrentMovementMode` "NewEnumerator3"))))

(fn `GetForwardSpeed`
  (returns (ForwardSpeed :type "Float (double-precision)"))
  (bind _bp_playerwheelchair (`self.BP_PlayerWheelchair`))
  (return (`KismetMathLibrary.Dot_VectorVector` (`self.GetVelocity` _bp_playerwheelchair) (`self.GetActorForwardVector` _bp_playerwheelchair))))

(fn `SetRearBrakeTorque`
  (params (TargetBrakeTorque :type "Float (double-precision)"))
  (bind _wheelchairvehiclemovementcomponent (`self.WheelchairVehicleMovementComponent`))
  (`ChaosWheeledVehicleMovementComponent.SetBrakeTorque` _wheelchairvehiclemovementcomponent TargetBrakeTorque 2)
  (`ChaosWheeledVehicleMovementComponent.SetBrakeTorque` _wheelchairvehiclemovementcomponent TargetBrakeTorque 3))

(fn `SetRearDriveTorque`
  (params (TargetDriveTorque :type "Float (double-precision)"))
  (bind _wheelchairvehiclemovementcomponent (`self.WheelchairVehicleMovementComponent`))
  (`ChaosWheeledVehicleMovementComponent.SetDriveTorque` _wheelchairvehiclemovementcomponent TargetDriveTorque 2)
  (`ChaosWheeledVehicleMovementComponent.SetDriveTorque` _wheelchairvehiclemovementcomponent TargetDriveTorque 3))

(fn `UserConstructionScript`)