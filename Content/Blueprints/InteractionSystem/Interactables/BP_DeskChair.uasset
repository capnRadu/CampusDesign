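; BP_DeskChair is an interactable desk chair that toggles between its starting position and a preset NewLocation.
; On Interact, it shows a fade widget if one is not already in the viewport, then teleports after a short delay, keeping rotation and scale.
; Moving to the new spot enables a linked actor (ActorToEnable), and returning to the original location disables it.
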(event `self.ReceiveBeginPlay`
  (bind _returnvalue_location (`KismetMathLibrary.BreakTransform` (`self.GetTransform`)))
  (`parent.ReceiveBeginPlay`)
  (set `self.OriginalLocation` _returnvalue_location))

(event `self.Interact`
  (bind (_returnvalue_location _returnvalue_rotation _returnvalue_scale) (`KismetMathLibrary.BreakTransform` (`self.GetTransform`)))
  (bind (_returnvalue_location_2 _returnvalue_rotation_2 _returnvalue_scale_2) (`KismetMathLibrary.BreakTransform` (`self.GetTransform`)))
  (bind _returnvalue_location_3 (`KismetMathLibrary.BreakTransform` (`self.GetTransform`)))
  (bind _fadewidget (`self.FadeWidget`))
  (`parent.Interact`)
  (if (not (`Widget.IsInViewport` _fadewidget))
    (`UserWidget.AddToViewport` _fadewidget 0)
    (`KismetSystemLibrary.Delay` 0.5)
    (if (`KismetMathLibrary.EqualExactly_VectorVector` _returnvalue_location_3 (`self.OriginalLocation`))
      (`self.K2_SetActorTransform` (`KismetMathLibrary.MakeTransform` (`self.NewLocation`) _returnvalue_rotation_2 _returnvalue_scale_2) false true)
      (`/Game/Blueprints/InteractionSystem/Interactables/BP_Seat.Enable` (`self.ActorToEnable`))
      (else
        (`self.K2_SetActorTransform` (`KismetMathLibrary.MakeTransform` (`self.OriginalLocation`) _returnvalue_rotation _returnvalue_scale) false true)
        (`/Game/Blueprints/InteractionSystem/Interactables/BP_Seat.Disable` (`self.ActorToEnable`))))))

(fn `UserConstructionScript`
  (`parent.UserConstructionScript`))