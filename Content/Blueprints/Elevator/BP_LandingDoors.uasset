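; Landing door Blueprint for an elevator that slides a pair of door meshes open and closed.
; Open and Close events each wait half a second, then play or reverse a shared timeline.
; The timeline's position track scales to a Y offset, moving the left and right doors in opposite directions in relative space.
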(event `Open`
  (`KismetSystemLibrary.Delay` 0.5)
  (`TimelineComponent.Play` (`self.ToggleLandingDoorsTimeline`)))

(event `Close`
  (`KismetSystemLibrary.Delay` 0.5)
  (`TimelineComponent.Reverse` (`self.ToggleLandingDoorsTimeline`)))

(fn `UserConstructionScript`)