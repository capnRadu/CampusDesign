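; BP_Goal is a quest goal actor in the world that completes a target quest when the player reaches it.
; On BeginPlay it caches whichever player pawn is in use, wheelchair or neurodivergent, and registers itself with BP_GameInstance.
; Overlapping its sphere completes the quest through the game instance if the goal is standalone, then destroys the actor on success.
; ActivateWaypoint reveals its direction arrow.
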(event `self.ReceiveBeginPlay`
  (bind _returnvalue (`Controller.K2_GetPawn` (`GameplayStatics.GetPlayerController` 0)))
  (`|ExecutionSequence`
    (:`then_0`
      (bind _asbp_player_wheelchair (cast `/Game/Blueprints/WheelchairController/BP_PlayerWheelchair` _returnvalue)
        (:`then`
          (set `self.PlayerWheelchair` _asbp_player_wheelchair))
        (:`CastFailed`
          (bind _asbp_player_neurodivergent (cast `/Game/Blueprints/NeurodivergentController/Blueprints/BP_PlayerNeurodivergent` _returnvalue))
          (set `self.PlayerNeurodivergent` _asbp_player_neurodivergent))))
    (:`then_1`
      (bind _asbp_game_instance (cast `/Game/Blueprints/GameInstances/BP_GameInstance` (`GameplayStatics.GetGameInstance`)))
      (set `self.GameInstance` _asbp_game_instance))
    (:`then_2`
      (`/Game/Blueprints/GameInstances/BP_GameInstance.RegisterSceneGoal` (`self.GameInstance`) self))))

(event `ActivateWaypoint`
  (bind _directionarrow (`self.DirectionArrow`))
  (if (not (`SceneComponent.bVisible` _directionarrow))
    (`SceneComponent.SetVisibility` _directionarrow true false)))

(event `self.Sphere.OnComponentBeginOverlap`
  (params (OverlappedComponent :type "PrimitiveComponent Object Reference") (OtherActor :type "Actor Object Reference") (OtherComp :type "PrimitiveComponent Object Reference") (OtherBodyIndex :type Integer) (bFromSweep :type Boolean) (SweepResult :type "HitResult Structure (by ref)"))
  (if (or (== OtherActor (`self.PlayerWheelchair`)) (== OtherActor (`self.PlayerNeurodivergent`)))
    (if (`self.IsStandaloneQuest`)
      (`self.TriggerCompleteQuest`))))

(event `TriggerCompleteQuest`
  (bind _questcompleted (`/Game/Blueprints/GameInstances/BP_GameInstance.CompleteQuest` (`self.GameInstance`) (`self.TargetQuestID`)))
  (if _questcompleted
    (`self.K2_DestroyActor`)))

(fn `UserConstructionScript`)