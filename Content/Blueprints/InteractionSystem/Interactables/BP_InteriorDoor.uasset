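; An interactable interior door that swings open and closed when the player interacts with it.
; The door caches the mesh's starting rotation, and each interaction plays or reverses the Rotate timeline, ignoring input while it is moving.
; The timeline lerps relative yaw from that rotation by the Direction offset, then updates IsOpen and the open/close prompt on finish.
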(event `self.ReceiveBeginPlay`
  (`parent.ReceiveBeginPlay`)
  (set `self.StartingRotation` (`SceneComponent.RelativeRotation` (`self.StaticMesh`))))

(event `/Game/Blueprints/InteractionSystem/BPI_Interact.Interact`
  (`parent.Interact`)
  (`self.Toggle`))

(event `Toggle`
  (if (`TimelineComponent.IsPlaying` (`self.Rotate`))
    _
    (elif (`self.IsOpen`)
      (`TimelineComponent.Reverse` (`self.Rotate`))
      (else
        (`TimelineComponent.PlayFromStart` (`self.Rotate`))))))

(fn `UserConstructionScript`
  (`parent.UserConstructionScript`))