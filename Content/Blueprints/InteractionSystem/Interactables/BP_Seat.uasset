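; BP_Seat is an interactable seat in the interaction system that can be switched on and off and shows a fade widget when used.
; Interact runs the parent logic, then adds the fade widget to the viewport if it is not already there.
; Enable and Disable toggle actor visibility, mesh query collision and the interact mark, with an option to start disabled at BeginPlay.
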(event `self.ReceiveBeginPlay`
  (`parent.ReceiveBeginPlay`)
  (if (`self.StartsDisabled`)
    (`self.Disable`)))

(event `self.Interact`
  (bind _fadewidget (`self.FadeWidget`))
  (`parent.Interact`)
  (if (not (`Widget.IsInViewport` _fadewidget))
    (`UserWidget.AddToViewport` _fadewidget 0)))

(event `Enable`
  (bind _interactmark (`self.InteractMark`))
  (`self.SetActorHiddenInGame` false)
  (`PrimitiveComponent.SetCollisionEnabled` (`self.StaticMesh`) "QueryOnly")
  (`/Game/Blueprints/Widgets/WBP_InteractMark.Show` _interactmark)
  (`WidgetComponent.SetWidget` (`self.Widget`) _interactmark))

(event `Disable`
  (`self.SetActorHiddenInGame` true)
  (`PrimitiveComponent.SetCollisionEnabled` (`self.StaticMesh`) "NoCollision")
  (`/Game/Blueprints/Widgets/WBP_InteractMark.Hide` (`self.InteractMark`)))

(fn `UserConstructionScript`
  (`parent.UserConstructionScript`))