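; BP_RevolvingDoor is a revolving door that spins at constant yaw speed while enabled for the wheelchair or neurodivergent player character.
; Either character entering its Sphere trigger starts rotation, and leaving stops it.
; A hit on the door mesh by either character halts it and starts a three-second timer.
; The timer resumes rotation if exactly one actor of either player class is still inside the Sphere.
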(event `self.ReceiveTick`
  (params (DeltaSeconds :type "Float (single-precision)"))
  (if (`self.CanRotate`)
    (`self.K2_AddActorLocalRotation` (`KismetMathLibrary.MakeRotator` 0.0 0.0 (* DeltaSeconds -50.0)))))

(event `self.SM_RevolvingDoor.OnComponentHit`
  (params (HitComponent :type "PrimitiveComponent Object Reference") (OtherActor :type "Actor Object Reference") (OtherComp :type "PrimitiveComponent Object Reference") (NormalImpulse :type "Vector Structure") (Hit :type "HitResult Structure (by ref)"))
  (cast `/Game/Blueprints/WheelchairController/BP_PlayerWheelchair` OtherActor
    (:`then`
      _)
    (:`CastFailed`
      (cast `/Game/Blueprints/NeurodivergentController/Blueprints/BP_PlayerNeurodivergent` OtherActor)))
  (set `self.CanRotate` false)
  (if (not (`KismetSystemLibrary.K2_IsValidTimerHandle` (`self.ResetTimer`)))
    (bind _returnvalue (`KismetSystemLibrary.K2_SetTimerDelegate` (delegate `ResetRotationState`) 3.0))
    (set `self.ResetTimer` _returnvalue)))

(event `ResetRotationState`
  (if (or (== (`KismetArrayLibrary.Array_Length` (`PrimitiveComponent.GetOverlappingActors` (`self.Sphere`) "/Game/Blueprints/NeurodivergentController/Blueprints/BP_PlayerNeurodivergent.BP_PlayerNeurodivergent_C")) 1) (== (`KismetArrayLibrary.Array_Length` (`PrimitiveComponent.GetOverlappingActors` (`self.Sphere`) "/Game/Blueprints/WheelchairController/BP_PlayerWheelchair.BP_PlayerWheelchair_C")) 1))
    (set `self.CanRotate` true)
    (`KismetSystemLibrary.K2_ClearAndInvalidateTimerHandle` (`self.ResetTimer`))))

(event `self.Sphere.OnComponentBeginOverlap`
  (params (OverlappedComponent :type "PrimitiveComponent Object Reference") (OtherActor :type "Actor Object Reference") (OtherComp :type "PrimitiveComponent Object Reference") (OtherBodyIndex :type Integer) (bFromSweep :type Boolean) (SweepResult :type "HitResult Structure (by ref)"))
  (cast `/Game/Blueprints/WheelchairController/BP_PlayerWheelchair` OtherActor
    (:`then`
      _)
    (:`CastFailed`
      (cast `/Game/Blueprints/NeurodivergentController/Blueprints/BP_PlayerNeurodivergent` OtherActor)))
  (set `self.CanRotate` true))

(event `self.Sphere.OnComponentEndOverlap`
  (params (OverlappedComponent :type "PrimitiveComponent Object Reference") (OtherActor :type "Actor Object Reference") (OtherComp :type "PrimitiveComponent Object Reference") (OtherBodyIndex :type Integer))
  (cast `/Game/Blueprints/WheelchairController/BP_PlayerWheelchair` OtherActor
    (:`then`
      _)
    (:`CastFailed`
      (cast `/Game/Blueprints/NeurodivergentController/Blueprints/BP_PlayerNeurodivergent` OtherActor)))
  (set `self.CanRotate` false))

(fn `UserConstructionScript`)