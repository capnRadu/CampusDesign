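; BP_EntranceDoor is an entrance door that swings open and closes itself again.
; Open plays the Rotate timeline, which lerps the static mesh's yaw 90 degrees negative from the rotation cached at BeginPlay.
; When fully open it sets IsOpen, which blocks further Open calls, and starts a timer that calls Close to reverse the timeline.
; IsOpen clears only once the reverse finishes.
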(event `self.ReceiveBeginPlay`
  (`parent.ReceiveBeginPlay`)
  (set `self.StartingRotation` (`SceneComponent.RelativeRotation` (`self.StaticMesh`))))

(event `Open`
  (if (not (`self.IsOpen`))
    (`TimelineComponent.PlayFromStart` (`self.Rotate`))))

(event `Close`
  (`TimelineComponent.Reverse` (`self.Rotate`)))

(fn `UserConstructionScript`)